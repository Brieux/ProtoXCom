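; Player controller for an XCom-style prototype that lets the player select units and order them to move or shoot.
; It gathers all BP_Unit actors at start and switches the controlled one through five hotkeys.
; A state toggle flips between Moving and Aiming, and the action input triggers movement or a shot through the unit's AIController_Unit, then refreshes the camera pawn's stats widget.
; Separate inputs adjust the PA committed to a shot.
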(event Custom|MoveUnit
  (Character|Jump (Variables|Default|GetControlledUnit))
  (bind _asaicontroller_unit (Utilities|Casting|CastToAIController_Unit (Pawn|GetController (Variables|Default|GetControlledUnit))))
  (Default|Moveto _asaicontroller_unit (Variables|/Game/ProtoXCom/AIController_Unit.AIController_Unit_C|GetDestination _asaicontroller_unit)))

(event Input|EnhancedActionEvents|EnhancedInputActionIA_ChangeStateOfCombat
  (params (ActionValue :type Boolean) (ElapsedSeconds :type Float%20%28double-precision%29) (TriggeredSeconds :type Float%20%28double-precision%29) (InputAction :type Input%20Action%20Object%20Reference :default "/Game/Input/IA_ChangeStateOfCombat.IA_ChangeStateOfCombat"))
  (bind _controlledunit (Variables|Default|GetControlledUnit))
  (bind _controlledunit_2 (Variables|Default|GetControlledUnit))
  (bind _controlledunit_3 (Variables|Default|GetControlledUnit))
  (bind _controlledunit_4 (Variables|Default|GetControlledUnit))
  (:Completed
    (Utilities|FlowControl|Sequence
      (:then_0
        (switch Utilities|FlowControl|Switch|SwitchonEnum_StateOfCombat (Variables|/Game/ProtoXCom/BP_Unit.BP_Unit_C|GetState _controlledunit_2)
          (:NewEnumerator0
            (Variables|/Game/ProtoXCom/BP_Unit.BP_Unit_C|SetState (Variables|Default|GetControlledUnit) "NewEnumerator1")
            (Variables|/Game/ProtoXCom/BP_Unit.BP_Unit_C|SetAbleToMove? _controlledunit_3 false)
            (bind _asaicontroller_unit (Utilities|Casting|CastToAIController_Unit (Pawn|GetController _controlledunit_4)))
            (Default|ClearPath _asaicontroller_unit)
            (Spline|ClearSplinePoints (Variables|/Game/ProtoXCom/BP_Unit.BP_Unit_C|GetSpline _controlledunit) true)
            (Default|ShowPA _controlledunit 0.0))
          (:NewEnumerator1
            (Variables|/Game/ProtoXCom/BP_Unit.BP_Unit_C|SetState _controlledunit_2 "NewEnumerator0")
            (Variables|/Game/ProtoXCom/BP_Unit.BP_Unit_C|SetAbleToMove? _controlledunit_3 true)
            (Default|ClearShowPA _controlledunit_4))))
      (:then_1
        (Development|PrintString (Utilities|String|EnumtoString (Variables|/Game/ProtoXCom/BP_Unit.BP_Unit_C|GetState (Variables|Default|GetControlledUnit))))))))

(event Input|EnhancedActionEvents|EnhancedInputActionIA_AddShootValue
  (params (ActionValue :type Boolean) (ElapsedSeconds :type Float%20%28double-precision%29) (TriggeredSeconds :type Float%20%28double-precision%29) (InputAction :type Input%20Action%20Object%20Reference :default "/Game/Input/IA_AddShootValue.IA_AddShootValue"))
  (bind _controlledunit (Variables|Default|GetControlledUnit))
  (:Completed
    (if (Variables|/Game/ProtoXCom/BP_Unit.BP_Unit_C|GetAbleToShoot? (Variables|Default|GetControlledUnit))
      (bind _result (Math|Integer|IncrementInt (Variables|/Game/ProtoXCom/BP_Unit.BP_Unit_C|GetPAShoot _controlledunit))
        (:%20%20
          (Variables|/Game/ProtoXCom/BP_Unit.BP_Unit_C|SetPAShoot _controlledunit (Math|Integer|Clamp(Integer) _result 1 (Variables|/Game/ProtoXCom/BP_Unit.BP_Unit_C|GetPA _controlledunit)))
          (Default|ShowPA (Variables|Default|GetControlledUnit) 0.0))))))

(event Input|EnhancedActionEvents|EnhancedInputActionIA_MinusShootValue
  (params (ActionValue :type Boolean) (ElapsedSeconds :type Float%20%28double-precision%29) (TriggeredSeconds :type Float%20%28double-precision%29) (InputAction :type Input%20Action%20Object%20Reference :default "/Game/Input/IA_MinusShootValue.IA_MinusShootValue"))
  (bind _controlledunit (Variables|Default|GetControlledUnit))
  (:Completed
    (if (Variables|/Game/ProtoXCom/BP_Unit.BP_Unit_C|GetAbleToShoot? (Variables|Default|GetControlledUnit))
      (bind _result (Math|Integer|DecrementInt (Variables|/Game/ProtoXCom/BP_Unit.BP_Unit_C|GetPAShoot _controlledunit))
        (:%20%20
          (Variables|/Game/ProtoXCom/BP_Unit.BP_Unit_C|SetPAShoot _controlledunit (Math|Integer|Clamp(Integer) _result 1 (Variables|/Game/ProtoXCom/BP_Unit.BP_Unit_C|GetPA _controlledunit)))
          (Default|ShowPA (Variables|Default|GetControlledUnit) 0.0))))))

(event Input|EnhancedActionEvents|EnhancedInputActionIA_SwitchControlledUnit_01
  (params (ActionValue :type Boolean) (ElapsedSeconds :type Float%20%28double-precision%29) (TriggeredSeconds :type Float%20%28double-precision%29) (InputAction :type Input%20Action%20Object%20Reference :default "/Game/Input/IA_SwitchControlledUnit_01.IA_SwitchControlledUnit_01"))
  (:Completed
    (if (>= (Utilities|Array|Length (Variables|Default|GetControlledTab)) 1)
      (CallFunction|SwitchControlledUnit))))

(event Input|EnhancedActionEvents|EnhancedInputActionIA_ActionUnit
  (params (ActionValue :type Boolean) (ElapsedSeconds :type Float%20%28double-precision%29) (TriggeredSeconds :type Float%20%28double-precision%29) (InputAction :type Input%20Action%20Object%20Reference :default "/Game/Input/IA_ActionUnit.IA_ActionUnit"))
  (bind _controlledunit (Variables|Default|GetControlledUnit))
  (bind _returnvalue (Pawn|GetController _controlledunit))
  (:Completed
    (switch Utilities|FlowControl|Switch|SwitchonEnum_StateOfCombat (Variables|/Game/ProtoXCom/BP_Unit.BP_Unit_C|GetState (Variables|Default|GetControlledUnit))
      (:NewEnumerator0
        (bind _asaicontroller_unit (Utilities|Casting|CastToAIController_Unit _returnvalue))
        (if (not (<= (Variables|/Game/ProtoXCom/AIController_Unit.AIController_Unit_C|GetActualPathCost _asaicontroller_unit) 1e+02))
          (CallFunction|MoveUnit)
          (bind _asbp_cam_pawn (Utilities|Casting|CastToBP_CamPawn (Pawn|GetControlledPawn) :!label _label))
          (Default|RefreshStat (Variables|/Game/ProtoXCom/BP_CamPawn.BP_CamPawn_C|GetWidget_Interface _asbp_cam_pawn) (Variables|Default|GetControlledIndex))))
      (:NewEnumerator1
        (bind _asaicontroller_unit_2 (Utilities|Casting|CastToAIController_Unit _returnvalue))
        (bind _enemyaimed (Variables|/Game/ProtoXCom/AIController_Unit.AIController_Unit_C|GetEnemyAimed _asaicontroller_unit_2)
          (:then
            (Default|ShootEnemyAfterValidate _asaicontroller_unit_2 _enemyaimed)
            (goto _label))
          (:else))))))

(event Input|EnhancedActionEvents|EnhancedInputActionIA_SwitchControlledUnit_02
  (params (ActionValue :type Boolean) (ElapsedSeconds :type Float%20%28double-precision%29) (TriggeredSeconds :type Float%20%28double-precision%29) (InputAction :type Input%20Action%20Object%20Reference :default "/Game/Input/IA_SwitchControlledUnit_02.IA_SwitchControlledUnit_02"))
  (:Completed
    (if (>= (Utilities|Array|Length (Variables|Default|GetControlledTab)) 2)
      (CallFunction|SwitchControlledUnit 1))))

(event Input|EnhancedActionEvents|EnhancedInputActionIA_SwitchControlledUnit_03
  (params (ActionValue :type Boolean) (ElapsedSeconds :type Float%20%28double-precision%29) (TriggeredSeconds :type Float%20%28double-precision%29) (InputAction :type Input%20Action%20Object%20Reference :default "/Game/Input/IA_SwitchControlledUnit_03.IA_SwitchControlledUnit_03"))
  (:Completed
    (if (>= (Utilities|Array|Length (Variables|Default|GetControlledTab)) 3)
      (CallFunction|SwitchControlledUnit 2))))

(event Input|EnhancedActionEvents|EnhancedInputActionIA_SwitchControlledUnit_04
  (params (ActionValue :type Boolean) (ElapsedSeconds :type Float%20%28double-precision%29) (TriggeredSeconds :type Float%20%28double-precision%29) (InputAction :type Input%20Action%20Object%20Reference :default "/Game/Input/IA_SwitchControlledUnit_04.IA_SwitchControlledUnit_04"))
  (:Completed
    (if (>= (Utilities|Array|Length (Variables|Default|GetControlledTab)) 4)
      (CallFunction|SwitchControlledUnit 3))))

(event Input|EnhancedActionEvents|EnhancedInputActionIA_SwitchControlledUnit_05
  (params (ActionValue :type Boolean) (ElapsedSeconds :type Float%20%28double-precision%29) (TriggeredSeconds :type Float%20%28double-precision%29) (InputAction :type Input%20Action%20Object%20Reference :default "/Game/Input/IA_SwitchControlledUnit_05.IA_SwitchControlledUnit_05"))
  (:Completed
    (if (>= (Utilities|Array|Length (Variables|Default|GetControlledTab)) 5)
      (CallFunction|SwitchControlledUnit 4))))

(event EventBeginPlay
  (Variables|Default|SetbShowMouseCursor true)
  (bind _outactors (Actor|GetAllActorsOfClass "/Game/ProtoXCom/BP_Unit.BP_Unit_C"))
  (bind _output_get (Variables|Default|SetControlledTab _outactors))
  (bind _output_get_2 (Variables|Default|SetControlledUnit (Utilities|Array|Get(acopy) _output_get (Variables|Default|GetControlledIndex))))
  (Variables|/Game/ProtoXCom/BP_Unit.BP_Unit_C|SetState _output_get_2 "NewEnumerator0"))

(event EventTick
  (params (DeltaSeconds :type Float%20%28single-precision%29)))

(fn ConstructionScript)

(fn SwitchControlledUnit
  (params (IndexToControl :type Integer))
  (Variables|/Game/ProtoXCom/BP_Unit.BP_Unit_C|SetState (Variables|Default|GetControlledUnit) "NewEnumerator2")
  (bind _output_get (Variables|Default|SetControlledUnit (Utilities|Array|Get(acopy) (Variables|Default|GetControlledTab) IndexToControl)))
  (Variables|/Game/ProtoXCom/BP_Unit.BP_Unit_C|SetState _output_get "NewEnumerator0")
  (Variables|Default|SetControlledIndex IndexToControl))