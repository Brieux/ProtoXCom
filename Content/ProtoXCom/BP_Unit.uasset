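; BP_Unit is a unit actor for an XCom-style prototype that previews movement paths, aim lines and their PA (likely action point) cost.
; ShowPath rebuilds a spline from the unit through the given points, setting points linear.
; ShowPA writes the TextRender by State: distance-scaled cost when moving, fixed shot cost when aiming, blank when inactive.
; CreateSplineAim draws a line to the enemy and enables shooting, which ClearAim reverts.
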(event Custom|ShowPath
  (params (PathPoint :type Array%20of%20Vectors))
  (bind _spline (Variables|Default|GetSpline))
  (Spline|ClearSplinePoints (Variables|Default|GetSpline) false)
  (Spline|AddSplinePoint (Variables|Default|GetSpline) (Transformation|GetActorLocation) "World" false)
  (for (_array_element _array_index) PathPoint
    (Spline|AddSplinePoint _spline _array_element "World" false)
    (Spline|SetSplinePointType _spline _array_index "Linear" false))
  (Spline|UpdateSpline _spline))

(event Custom|ShowPA
  (params (Cost :type Float%20%28double-precision%29))
  (Rendering|Components|TextRender|SetText (Variables|Default|GetTextRender) (Utilities|Select :Index (Variables|Default|GetState) :NewEnumerator0 (Utilities|Text|ToText(Integer) (Math|Float|Truncate (/ Cost 1e+02))) :NewEnumerator1 (Utilities|Text|ToText(Integer) (Variables|Default|GetPAShoot)) :NewEnumerator2 "")))

(event Custom|CreateSplineAim
  (params (EnemyLoc :type Vector))
  (Spline|AddSplinePoint (Variables|Default|GetSpline) (Transformation|GetActorLocation) "World" true)
  (Spline|AddSplinePoint (Variables|Default|GetSpline) EnemyLoc "World" true)
  (Variables|Default|SetAbleToShoot? true)
  (Variables|Default|SetPAShoot 1)
  (CallFunction|ShowPA 0.0))

(event Custom|ClearAim
  (Spline|ClearSplinePoints (Variables|Default|GetSpline) true)
  (Variables|Default|SetAbleToShoot? false)
  (CallFunction|ClearShowPA))

(event Custom|ClearShowPA
  (Rendering|Components|TextRender|SetText (Variables|Default|GetTextRender) (Variables|Default|GetDefaultText))
  (Variables|Default|SetPAShoot 1))

(event EventBeginPlay)

(event Collision|EventActorBeginOverlap
  (params (OtherActor :type Actor%20Object%20Reference)))

(fn ConstructionScript)