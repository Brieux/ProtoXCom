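; BP_CamPawn is the player-possessed camera pawn of an XCom-style prototype, with planar movement and fixed 90-degree turns.
; On possession it adds the IMC_Control Enhanced Input context, and on BeginPlay it shows WID_Interface.
; Movement input follows the actor's forward and right vectors, while left/right timelines animate yaw steps from the starting rotation.
; CanMove and CanRotate flags keep movement and turning exclusive; free-rotation nodes are unconnected.
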(event Input|EnhancedActionEvents|EnhancedInputActionIA_MoveCamFront
  (params (ActionValue :type Float%20%28double-precision%29) (ElapsedSeconds :type Float%20%28double-precision%29) (TriggeredSeconds :type Float%20%28double-precision%29) (InputAction :type Input%20Action%20Object%20Reference :default "/Game/Input/IA_MoveCamFront.IA_MoveCamFront"))
  ;[0.5677 0.5618 0.5618 1 58] Movement/Rotation
  ;;[0.0787 1 0] MoveCam
  (:Triggered
    (Variables|Default|SetCanRotate? false :!label _label)
    (if (Variables|Default|GetCanMove?)
      (Pawn|Input|AddMovementInput (Transformation|GetActorForwardVector) (* ActionValue (Variables|Default|GetSpeed)) false)))
  (:Started
    (goto _label))
  (:Completed
    (Variables|Default|SetCanRotate? true)))

(event Input|EnhancedActionEvents|EnhancedInputActionIA_MoveCamRight
  (params (ActionValue :type Float%20%28double-precision%29) (ElapsedSeconds :type Float%20%28double-precision%29) (TriggeredSeconds :type Float%20%28double-precision%29) (InputAction :type Input%20Action%20Object%20Reference :default "/Game/Input/IA_MoveCamRight.IA_MoveCamRight"))
  ;[0.5677 0.5618 0.5618 1 58] Movement/Rotation
  ;;[0.0787 1 0] MoveCam
  (:Triggered
    (Variables|Default|SetCanRotate? false :!label _label)
    (if (Variables|Default|GetCanMove?)
      (Pawn|Input|AddMovementInput (Transformation|GetActorRightVector) (* ActionValue (Variables|Default|GetSpeed)) false)))
  (:Started
    (goto _label))
  (:Completed
    (Variables|Default|SetCanRotate? true)))

(event Input|EnhancedActionEvents|EnhancedInputActionIA_RotateCam
  (params (ActionValue :type Vector%202D%20Structure) (ElapsedSeconds :type Float%20%28double-precision%29) (TriggeredSeconds :type Float%20%28double-precision%29) (InputAction :type Input%20Action%20Object%20Reference :default "/Game/Input/IA_RotateCam.IA_RotateCam"))
  ;[0.5677 0.5618 0.5618 1 58] Movement/Rotation
  ;;[1 0 0.2052] RotateLibre
)

(event Input|EnhancedActionEvents|EnhancedInputActionIA_RotateCamFixLeft
  (params (ActionValue :type Boolean) (ElapsedSeconds :type Float%20%28double-precision%29) (TriggeredSeconds :type Float%20%28double-precision%29) (InputAction :type Input%20Action%20Object%20Reference :default "/Game/Input/IA_RotateCamFixLeft.IA_RotateCamFixLeft"))
  ;[0.5677 0.5618 0.5618 1 58] Movement/Rotation
  ;;[0 0.5052 1] RotateFixe
  (:Completed
    (if (Variables|Default|GetCanRotate?)
      (Variables|Default|SetCanMove? false)
      (Variables|Default|SetCanRotate? false)
      (Variables|Default|SetInitialRotation (Transformation|GetActorRotation))
      (Components|Timeline|SetPlayRate (Variables|Default|GetRotateLEft) (Variables|Default|GetPlayrate))
      (bind _newtrack_0 (Timeline|RotateLeft PlayFromStart)
        (:Update
          (Transformation|SetActorRotation (Math|Rotator|MakeRotator (.roll (Variables|Default|GetInitialRotation)) (.pitch (Variables|Default|GetInitialRotation)) (- (.yaw (Variables|Default|GetInitialRotation)) (Math|Float|Lerp 0.0 9e+01 _newtrack_0)))))
        (:Finished
          (Variables|Default|SetCanRotate? true)
          (Variables|Default|SetCanMove? true))))))

(event Input|EnhancedActionEvents|EnhancedInputActionIA_RotateCamFixRight
  (params (ActionValue :type Boolean) (ElapsedSeconds :type Float%20%28double-precision%29) (TriggeredSeconds :type Float%20%28double-precision%29) (InputAction :type Input%20Action%20Object%20Reference :default "/Game/Input/IA_RotateCamFixRight.IA_RotateCamFixRight"))
  ;[0.5677 0.5618 0.5618 1 58] Movement/Rotation
  ;;[0 0.5052 1] RotateFixe
  (:Completed
    (if (Variables|Default|GetCanRotate?)
      (Variables|Default|SetCanMove? false)
      (Variables|Default|SetCanRotate? false)
      (Variables|Default|SetInitialRotation (Transformation|GetActorRotation))
      (Components|Timeline|SetPlayRate (Variables|Default|GetRotateRight) (Variables|Default|GetPlayrate))
      (bind _newtrack_0 (Timeline|RotateRight PlayFromStart)
        (:Update
          (Transformation|SetActorRotation (Math|Rotator|MakeRotator (.roll (Variables|Default|GetInitialRotation)) (.pitch (Variables|Default|GetInitialRotation)) (+ (.yaw (Variables|Default|GetInitialRotation)) (Math|Float|Lerp 0.0 9e+01 _newtrack_0)))))
        (:Finished
          (Variables|Default|SetCanRotate? true)
          (Variables|Default|SetCanMove? true))))))

(event Collision|EventActorBeginOverlap
  (params (OtherActor :type Actor%20Object%20Reference))
  ;[0.5677 0.5618 0.5618 1 58] Movement/Rotation
)

(event EventTick
  (params (DeltaSeconds :type Float%20%28single-precision%29)))

(event EventPossessed
  (params (NewController :type Controller%20Object%20Reference))
  (bind _asbp_player_controller_xcom (Utilities|Casting|CastToBP_PlayerControllerXCom NewController))
  (Input|AddMappingContext (PlayerController|LocalPlayerSubsystems|GetEnhancedInputLocalPlayerSubsystem _asbp_player_controller_xcom) "/Game/Input/IMC_Control.IMC_Control" 0 "(bIgnoreAllPressedKeysUntilRelease=True,bForceImmediately=False)"))

(event EventBeginPlay
  (bind _returnvalue (UserInterface|CreateWidget "/Game/ProtoXCom/WID_Interface.WID_Interface_C"))
  (bind _output_get (Variables|Default|SetWidget_Interface _returnvalue))
  (UserInterface|Viewport|AddtoViewport _output_get 0))

(fn ConstructionScript)