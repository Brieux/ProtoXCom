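; BP_Enemy is an enemy actor for the XCom-style prototype that holds hit points (PV) and can display them.
; ShowPV writes the current PV to the PVToRender text, and ClearPV blanks it.
; ReceiveDammage subtracts damage from PV without refreshing the text, clamping the value or handling death.
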(event Custom|ShowPV
  (Rendering|Components|TextRender|SetText (Variables|Default|GetPVToRender) (Utilities|Text|ToText(Integer) (Variables|Default|GetPV))))

(event Custom|ClearPV
  (Rendering|Components|TextRender|SetText (Variables|Default|GetPVToRender) (Utilities|Text|ToText(String) "")))

(event Custom|ReceiveDammage
  (params (Dammage :type Integer))
  (Variables|Default|SetPV (- (Variables|Default|GetPV) Dammage)))

(event EventBeginPlay)

(event Collision|EventActorBeginOverlap
  (params (OtherActor :type Actor%20Object%20Reference)))

(event EventTick
  (params (DeltaSeconds :type Float%20%28single-precision%29)))

(fn ConstructionScript)