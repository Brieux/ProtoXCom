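; GM_XCom is the game mode for an XCom prototype that alternates turns between the player and the AI.
; ChangeTurn increments a turn counter and uses its parity to pick the side, printing whose turn it is.
; Even turns call BeginTurn on the first player's BP_PlayerControllerXCom, and odd turns call EndTurn on it.
; The AI turn has no further logic in this Blueprint.
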(event Custom|ChangeTurn
  (bind _result (Math|Integer|IncrementInt (Variables|Default|GetTurn))
    (:%20%20
      (bind _output_get (Variables|Default|SetTurn _result))
      (if (== (Math|Integer|%(Integer) _output_get 2) 0)
        (Development|PrintString "Player Turn")
        (bind _asbp_player_controller_xcom (Utilities|Casting|CastToBP_PlayerControllerXCom (Game|GetPlayerController 0)))
        (Default|BeginTurn _asbp_player_controller_xcom)
        (else
          (Development|PrintString "IA Turn")
          (bind _asbp_player_controller_xcom_2 (Utilities|Casting|CastToBP_PlayerControllerXCom (Game|GetPlayerController 0)))
          (Default|EndTurn _asbp_player_controller_xcom_2))))))

(event EventBeginPlay)

(event EventTick
  (params (DeltaSeconds :type Float%20%28single-precision%29)))

(fn ConstructionScript)